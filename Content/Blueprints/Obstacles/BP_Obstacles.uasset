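; Obstacle actor that damages the sprite character when hit.
; The construction script sets the Obstacle component's sprite from ObstacleType, covering rock, clam, cloud and fish variants in one Blueprint.
; On Hit, it casts the other actor to BP_SpriteCharacter and calls DamageHealth with a fixed damage amount.
; A DoOnce with no reset limits each obstacle instance to dealing damage a single time.
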(event Collision|EventHit
  (params (MyComp :type Primitive%20Component%20Object%20Reference) (Other :type Actor%20Object%20Reference) (OtherComp :type Primitive%20Component%20Object%20Reference) (bSelfMoved :type Boolean) (HitLocation :type Vector :default "0, 0, 0") (HitNormal :type Vector :default "0, 0, 0") (NormalImpulse :type Vector :default "0, 0, 0") (Hit :type Hit%20Result%20Structure%20%28by%20ref%29))
  (bind _asbp_sprite_character (Utilities|Casting|CastToBP_SpriteCharacter Other))
  (Utilities|FlowControl|DoOnce false
    (:Completed
      (Default|DamageHealth _asbp_sprite_character (Variables|/Game/Blueprints/character/BP_SpriteCharacter.BP_SpriteCharacter_C|GetCurrentHealth _asbp_sprite_character) 1e+01))))

(fn ConstructionScript
  (bind _obstacle (Variables|Default|Getobstacle))
  (switch Utilities|FlowControl|Switch|SwitchonEObstacle (Variables|Default|GetObstacleType)
    (:NewEnumerator0
      (Rendering|Components|Sprite|SetSprite _obstacle "/Game/Sprites/Obstacles/rock_Sprite.rock_Sprite"))
    (:NewEnumerator1
      (Rendering|Components|Sprite|SetSprite _obstacle "/Game/Sprites/Obstacles/clam_Sprite.clam_Sprite"))
    (:NewEnumerator2
      (Rendering|Components|Sprite|SetSprite _obstacle "/Game/Sprites/Obstacles/cloud_Sprite.cloud_Sprite"))
    (:NewEnumerator3
      (Rendering|Components|Sprite|SetSprite _obstacle "/Game/Sprites/Obstacles/fish_Sprite.fish_Sprite"))))