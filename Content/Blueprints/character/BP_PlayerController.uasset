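; Player controller that owns the HUD overlay and handles the player's death screen.
; On BeginPlay it plays a game-start sound and creates and shows the WB_Info_Overlay widget.
; UpdateHealthBar forwards health values to the overlay.
; When health reaches zero it pauses the game, plays a death sound, shows WB_Death_Screen and switches to mouse-driven UI-only input.
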(event Custom|UpdateHealthBar
  (params (CurrentHealth :type Float%20%28double-precision%29) (MaxHealth :type Float%20%28double-precision%29))
  (bind _returnvalue (Game|GetPlayerController 0))
  (Default|SetHealthBarInfo (Variables|Default|GetWB_Info) CurrentHealth MaxHealth)
  (if (<= CurrentHealth 0.0)
    (Game|SetGamePaused true)
    (Audio|PlaySound2D "/Game/music/sounds/Death.Death" 1.0 1.0 0.0 0 0)
    (bind _returnvalue_2 (UserInterface|CreateWidget "/Game/UI/WB_Death_Screen.WB_Death_Screen_C"))
    (UserInterface|Viewport|AddtoViewport _returnvalue_2 0)
    (Variables|/Script/Engine.PlayerController|SetbShowMouseCursor _returnvalue true)
    (Input|SetInputModeUIOnly _returnvalue 0 "DoNotLock" false)))

(event EventBeginPlay
  (Audio|PlaySound2D "/Game/music/sounds/game-start-6104.game-start-6104" 1.0 1.0 0.0 0 0)
  (bind _returnvalue (UserInterface|CreateWidget "/Game/UI/WB_Info_Overlay.WB_Info_Overlay_C"))
  (bind _output_get (Variables|Default|SetWB_Info _returnvalue))
  (UserInterface|Viewport|AddtoViewport _output_get 0))

(fn ConstructionScript)